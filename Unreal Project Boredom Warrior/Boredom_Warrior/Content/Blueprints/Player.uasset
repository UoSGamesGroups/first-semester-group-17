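; Player character Blueprint with side-on movement along world X, jumping, wall jumping and projectile firing.
; Pressing jump while airborne line-traces through the capsule along the forward axis, launching the character away from a hit wall or falling back to a jump limited by JumpCount.
; Landing resets that count, Fire spawns Projectile_BP at ProjectileSpawn, and BeginPlay adds the GameHUD widget and initializes current health.
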(event Custom|WallJump
  (bind _returnvalue (Transformation|GetActorForwardVector))
  ;[1 1 1] Wall Jump
  (bind (_outhit _returnvalue_2) (Collision|LineTraceByChannel (- (Transformation|GetActorLocation) (* _returnvalue (+ (Components|Capsule|GetScaledCapsuleRadius (Variables|Collision|GetCapsuleComponent)) 15.0))) (+ (Transformation|GetActorLocation) (* _returnvalue (+ (Components|Capsule|GetScaledCapsuleRadius (Variables|Collision|GetCapsuleComponent)) 15.0))) "TraceTypeQuery1" true 0 "None"))
  (if _returnvalue_2
    (Character|LaunchCharacter (Math|Vector|MakeVector (* (Math|Float|Sign(Float) (- (.x (Transformation|GetActorLocation)) (.x (.Location (Collision|BreakHitResult _outhit))))) 4.5e+02) 0.0 (Variables|/Script/Engine.CharacterMovementComponent|GetJumpZVelocity (Variables|Character|GetCharacterMovement))) true true)
    (elif (<= (Variables|Default|GetJumpCount) 1)
      (Character|Jump)
      (Variables|Default|SetJumpCount (+ (Variables|Default|GetJumpCount) 1)))))

(event EventBeginPlay
  (bind _returnvalue (UserInterface|CreateWidget "/Game/HUD/gameHUD.gameHUD_C"))
  (bind _output_get (Variables|Default|SetNewVar_0 _returnvalue))
  (UserInterface|Viewport|AddtoViewport _output_get 0)
  (bind _asplayer (Utilities|Casting|CastToPlayer (Game|Player|GetPlayerPawn 0)))
  (Variables|Default|SetHealthCurrent (Variables|Default|GetNewVar_3)))

(event EventOnLanded
  (params (Hit :type Hit%20Result%20Structure%20%28by%20ref%29))
  ;[1 1 1] Grounded Check
  (Variables|Default|SetJumpCount 0))

(event Input|ActionEvents|InputActionJump
  (params (Key :type Key%20Structure :default "AnyKey"))
  ;[1 1 1] Jumping
  (:Pressed
    (if (AI|Components|NavMovement|IsFalling (Variables|Character|GetCharacterMovement))
      (CallFunction|WallJump)
      (else
        (Character|Jump)
        (Variables|Default|SetJumpCount (+ (Variables|Default|GetJumpCount) 1)))))
  (:Released
    (Character|StopJumping)))

(event Input|ActionEvents|InputActionFire
  (params (Key :type Key%20Structure :default "AnyKey"))
  (:Pressed
    (Game|SpawnActorfromClass "/Game/Blueprints/Projectile_BP.Projectile_BP_C" (Transformation|GetWorldTransform (Variables|Default|GetProjectileSpawn)) "Undefined" 0 0)))

(event Input|AxisEvents|InputAxisRight
  (params (AxisValue :type Float%20%28single-precision%29))
  ;[1 1 1] Movement
  (Pawn|Input|AddMovementInput "1.000000, 0, 0" AxisValue false))

(fn ConstructionScript
  (Variables|/Script/Engine.CharacterMovementComponent|SetJumpZVelocity (Variables|Character|GetCharacterMovement) 5e+01)
  (Variables|Default|SetJumpMaxHoldTime 0.3)
  (Variables|Default|SetJumpCount 0))